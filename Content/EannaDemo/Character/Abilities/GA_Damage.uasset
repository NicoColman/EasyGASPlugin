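; GA_Damage is a Gameplay Ability that damages actors entering a box detection area while its input is held.
; On activation, a custom box overlap task with debug enabled runs alongside a wait for input release, which ends the ability.
; Each overlap's target data yields actors, and for each one the ability builds damage params from class defaults, then calls ApplyDamageEffect with DamageValues.
; An unconnected node for setting DamageValues notes that GAS_AttributeSet reads them.
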(event `self.K2_ActivateAbility`
  (`AbilityTask_WaitInputRelease.WaitInputRelease` false
    (:`then`
      (bind (_asynctaskproxy _datahandle) (`GASATask_CustomShapeOverlap.BP_DetectCustomBoxOverlap` :`BoxExtent` (`self.Box Extent`) :`CollisionChannel` (`self.Collision Channel`) :`bIgnoreSelf` false :`SceneToAttach` null :`bDebug` true)
        (:`OnBeginOverlap`
          (for _array_element (`AbilitySystemBlueprintLibrary.GetActorsFromTargetData` _datahandle)
            (`self.MakeDamageEffectParamsFromClassDefaults` _array_element)
            (`GAS_BlueprintFunctionLibrary.ApplyDamageEffect` (`self.DamageValues`) (struct))))))
    (:`OnRelease`
      (`self.K2_EndAbility`))))

(event `self.K2_OnEndAbility`
  (params (bWasCancelled :type Boolean)))